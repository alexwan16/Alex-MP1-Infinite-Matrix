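; BP_Monster is an enemy actor that damages the player on contact and can be shot for score.
; All logic runs from the Monster component's hit event, and the monster destroys itself on hitting either a player or a projectile.
; A BP_Player hit subtracts clamped health, then shows a HurtScreen widget, or flags death and displays restart at zero.
; A BP_Projectile hit increments the Score on the BP_Player found in the world.
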(event OnComponentHit(Monster)
  (params (HitComponent :type Primitive%20Component%20Object%20Reference) (OtherActor :type Actor%20Object%20Reference) (OtherComp :type Primitive%20Component%20Object%20Reference) (NormalImpulse :type Vector :default "0, 0, 0") (Hit :type Hit%20Result%20Structure%20%28by%20ref%29))
  (bind _asbp_player (Utilities|Casting|CastToBP_Player OtherActor)
    (:then
      (Utilities|FlowControl|Sequence
        (:then_0
          (Actor|DestroyActor))
        (:then_1
          (bind _output_get (Variables|/Game/InfiniteMatrix/Blueprints/BP_Player.BP_Player_C|SetHealth _asbp_player (Math|Float|Clamp(Float) (+ (Variables|/Game/InfiniteMatrix/Blueprints/BP_Player.BP_Player_C|GetHealth _asbp_player) -2e+01) 0.0 1e+02)))
          (if (== _output_get 0.0)
            (Variables|/Game/InfiniteMatrix/Blueprints/BP_Player.BP_Player_C|SetIsDead _asbp_player true)
            (Default|DisplayRestart _asbp_player)
            (else
              (bind _returnvalue (UserInterface|CreateWidget "/Game/InfiniteMatrix/UI/HurtScreen.HurtScreen_C"))
              (UserInterface|Viewport|AddtoViewport _returnvalue 0))))))
    (:CastFailed
      (Utilities|Casting|CastToBP_Projectile OtherActor)
      (Actor|DestroyActor)
      (bind _returnvalue_2 (Actor|GetActorOfClass "/Game/InfiniteMatrix/Blueprints/BP_Player.BP_Player_C"))
      (Variables|/Game/InfiniteMatrix/Blueprints/BP_Player.BP_Player_C|SetScore _returnvalue_2 (+ (Variables|/Game/InfiniteMatrix/Blueprints/BP_Player.BP_Player_C|GetScore _returnvalue_2) 1)))))

(event EventBeginPlay)

(event Collision|EventActorBeginOverlap
  (params (OtherActor :type Actor%20Object%20Reference)))

(event EventTick
  (params (DeltaSeconds :type Float%20%28single-precision%29)))

(fn ConstructionScript)